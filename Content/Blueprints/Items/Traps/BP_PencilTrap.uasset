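; BP_PencilTrap is a trap whose Trap component shuttles endlessly back and forth between two checkpoint components.
; BeginPlay fills the checkpoint array, places Trap at the first and starts GoToCheckpoint, a latent loop of eased MoveComponentTo, short pause and wrapping index increment.
; Tick snaps InteractableArea to Trap's world location so the interaction zone follows the moving trap.
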(event `self.ReceiveBeginPlay`
  (bind _firstcheckpoint (`self.FirstCheckpoint`))
  (`parent.ReceiveBeginPlay`)
  (`KismetArrayLibrary.Array_Add` (`self.Checkpoints`) _firstcheckpoint)
  (`KismetArrayLibrary.Array_Add` (`self.Checkpoints`) (`self.SecondCheckpoint`))
  (`SceneComponent.K2_SetWorldLocation` (`self.Trap`) (`SceneComponent.K2_GetComponentLocation` _firstcheckpoint) false false)
  (set `self.NextCheckpointIndex` 1)
  (`self.GoToCheckpoint`))

(event `self.ReceiveTick`
  (params (DeltaSeconds :type "Float (single-precision)"))
  (`parent.ReceiveTick` DeltaSeconds)
  (`SceneComponent.K2_SetWorldLocation` (`self.InteractableArea`) (`SceneComponent.K2_GetComponentLocation` (`self.Trap`)) false false))

(event `GoToCheckpoint`
  (`KismetSystemLibrary.MoveComponentTo` (`self.Trap`) (`SceneComponent.RelativeLocation` (`|GetArrayItem` (`self.Checkpoints`) (`self.NextCheckpointIndex`))) (struct) true true 3.0 :!label _label)
  (`KismetSystemLibrary.Delay` 1.0)
  (bind _result (`/Engine/EditorBlueprintResources/StandardMacros.IncrementInt` (`self.NextCheckpointIndex`))
    (:`  `
      (if (>= _result (`KismetArrayLibrary.Array_Length` (`self.Checkpoints`)))
        (set `self.NextCheckpointIndex` 0)
        (goto _label)
        (else
          (goto _label))))))

(fn `UserConstructionScript`
  (`parent.UserConstructionScript`))