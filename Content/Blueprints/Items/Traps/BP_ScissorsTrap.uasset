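; BP_ScissorsTrap is a trap whose Trap component patrols endlessly back and forth between two checkpoint components.
; On BeginPlay it fills the Checkpoints array, places the trap at the first one and starts the Patrolling loop.
; Each leg snaps the trap to the current checkpoint's rotation, moves it to the next with MoveComponentTo, then waits briefly before repeating.
; The graph contains no overlap or damage logic.
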(event `self.ReceiveBeginPlay`
  (bind _firstcheckpoint (`self.FirstCheckpoint`))
  (`parent.ReceiveBeginPlay`)
  (`KismetArrayLibrary.Array_Add` (`self.Checkpoints`) _firstcheckpoint)
  (`KismetArrayLibrary.Array_Add` (`self.Checkpoints`) (`self.SecondCheckpoint`))
  (`SceneComponent.K2_SetWorldLocation` (`self.Trap`) (`SceneComponent.K2_GetComponentLocation` _firstcheckpoint) false false)
  (`self.Patrolling`))

(event `Patrolling`
  (bind _trap (`self.Trap`))
  (`SceneComponent.K2_SetRelativeRotation` (`self.Trap`) (`SceneComponent.RelativeRotation` (`|GetArrayItem` (`self.Checkpoints`) (`self.NextCheckpointIndex`))) false false :!label _label)
  (bind _result (`/Engine/EditorBlueprintResources/StandardMacros.IncrementInt` (`self.NextCheckpointIndex`))
    (:`  `
      (if (>= _result (`KismetArrayLibrary.Array_Length` (`self.Checkpoints`)))
        (set `self.NextCheckpointIndex` 0))
      (`KismetSystemLibrary.MoveComponentTo` _trap (`SceneComponent.RelativeLocation` (`|GetArrayItem` (`self.Checkpoints`) (`self.NextCheckpointIndex`))) (`SceneComponent.RelativeRotation` _trap) false false 2.0)
      (`KismetSystemLibrary.Delay` 1.0)
      (goto _label))))

(fn `UserConstructionScript`
  (`parent.UserConstructionScript`))