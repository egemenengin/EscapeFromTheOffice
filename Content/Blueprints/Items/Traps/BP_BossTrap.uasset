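; Boss trap actor that sweeps its Trap component back and forth through a 180-degree arc, keeping the boss animation in sync.
; While IsRotating is set, Tick calls RotateBoss, which applies a fixed local rotation step and flips direction at each limit, so speed depends on frame rate.
; The current angle is pushed to the boss's BossAnimInst, cached on BeginPlay, as CurrentRotateAmount.
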(event `self.ReceiveBeginPlay`
  (`parent.ReceiveBeginPlay`)
  (bind _asboss_anim_inst (cast `/Game/Animations/Item/Boss/BossAnimInst` (`SkeletalMeshComponent.GetAnimInstance` (`self.Boss`))))
  (bind _output_get (set `self.BossAnimInst` _asboss_anim_inst))
  (set `/Game/Animations/Item/Boss/BossAnimInst.CurrentRotateAmount` (`self.RotateAmount`) _output_get))

(event `self.ReceiveTick`
  (params (DeltaSeconds :type "Float (single-precision)"))
  (`parent.ReceiveTick` DeltaSeconds)
  (if (`self.bIsRotating`)
    (`self.RotateBoss`)
    (set `/Game/Animations/Item/Boss/BossAnimInst.CurrentRotateAmount` (`self.RotateAmount`) (`self.BossAnimInst`))))

(fn `RotateBoss`
  (if (`self.bRotateRight`)
    (if (< (`self.RotateAmount`) 180.0)
      (`SceneComponent.K2_AddLocalRotation` (`self.Trap`) (struct :`Yaw` 0.5) false false)
      (set `self.RotateAmount` (+ (`self.RotateAmount`) 0.5))
      (else
        (set `self.bRotateRight` false)))
    (elif (> (`self.RotateAmount`) 0.0)
      (`SceneComponent.K2_AddLocalRotation` (`self.Trap`) (struct :`Yaw` -0.5) false false)
      (set `self.RotateAmount` (- (`self.RotateAmount`) 0.5))
      (else
        (set `self.bRotateRight` true)))))

(fn `UserConstructionScript`
  (`parent.UserConstructionScript`))