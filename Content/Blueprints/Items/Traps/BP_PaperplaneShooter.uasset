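; BP_PaperplaneShooter is a trap that repeatedly launches paperplane projectiles.
; Every Tick calls Shoot, which, while CanShoot is true, spawns a BP_PaperplaneTrap at SpawnPoint with a configurable lifetime and pushes it horizontally along the spawn point's right vector.
; A timer then flips CanShoot back after a fixed cooldown, pacing the shots.
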(event `self.ReceiveTick`
  (params (DeltaSeconds :type "Float (single-precision)"))
  (`parent.ReceiveTick` DeltaSeconds)
  (`self.Shoot`))

(fn `SetCanShoot`
  (set `self.bCanShoot` (not (`self.bCanShoot`))))

(fn `Shoot`
  (bind _spawnpoint (`self.SpawnPoint`))
  (if (`self.bCanShoot`)
    (set `self.bCanShoot` false)
    (bind _returnvalue (`|SpawnActorFromClass` "/Game/Blueprints/Items/Traps/BP_PaperplaneTrap.BP_PaperplaneTrap_C" (`SceneComponent.K2_GetComponentToWorld` _spawnpoint) "Undefined" "OverrideRootScale" null (`self.AmmoLifeTime`) null))
    (`PrimitiveComponent.AddForce` (`/Game/Blueprints/Items/Traps/BP_TrapBase.Trap` _returnvalue) (* (`SceneComponent.GetRightVector` _spawnpoint) (20000.0 20000.0 0.0)) "None" false)
    (`KismetSystemLibrary.K2_SetTimer` null "SetCanShoot" 2.5)))

(fn `UserConstructionScript`
  (`parent.UserConstructionScript`))