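; BP_LevelEnd is a level exit trigger that ends the current floor when the player reaches it.
; Overlap on its InteractableArea component checks that the other actor is a BP_PlayerCharacter.
; It then calls SetGameStatus on BP_EFTOGameMode with a new status and its FloorNumber as the finished level, leaving the outcome to the game mode.
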(event `self.InteractableArea.OnComponentBeginOverlap`
  (params (OverlappedComponent :type "PrimitiveComponent Object Reference") (OtherActor :type "Actor Object Reference") (OtherComp :type "PrimitiveComponent Object Reference") (OtherBodyIndex :type Integer) (bFromSweep :type Boolean) (SweepResult :type "HitResult Structure (by ref)"))
  (`/Engine/EditorBlueprintResources/StandardMacros.IsValid` OtherActor
    (:`Is Valid`
      (cast `/Game/Blueprints/Player/BP_PlayerCharacter` OtherActor)
      (bind _asbp_eftogame_mode (cast `/Game/Blueprints/BP_EFTOGameMode` (`GameplayStatics.GetGameMode`)))
      (`/Game/Blueprints/BP_EFTOGameMode.SetGameStatus` _asbp_eftogame_mode "NewEnumerator2" (`self.FloorNumber`)))))

(fn `UserConstructionScript`
  (`parent.UserConstructionScript`))