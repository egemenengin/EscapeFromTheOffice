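; BP_InformativeItem is an item Blueprint with an information widget and an area that detects the player.
; On BeginPlay it passes itself to the WBP_InfoWidget hosted by InformationWidget as that widget's item reference.
; InformativeDetectableArea overlap events send +1 on enter and -1 on exit to BP_PlayerCharacter's OverlappedInteractablesHandler, reporting changes in overlapped interactables.
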(event `self.ReceiveBeginPlay`
  (`parent.ReceiveBeginPlay`)
  (bind _aswbp_info_widget (cast `/Game/Blueprints/HUDs/Gameplay/WBP_InfoWidget` (`WidgetComponent.GetUserWidgetObject` (`self.InformationWidget`))))
  (set `/Game/Blueprints/HUDs/Gameplay/WBP_InfoWidget.ItemReference` self _aswbp_info_widget))

(event `self.InformativeDetectableArea.OnComponentBeginOverlap`
  (params (OverlappedComponent :type "PrimitiveComponent Object Reference") (OtherActor :type "Actor Object Reference") (OtherComp :type "PrimitiveComponent Object Reference") (OtherBodyIndex :type Integer) (bFromSweep :type Boolean) (SweepResult :type "HitResult Structure (by ref)"))
  (`/Engine/EditorBlueprintResources/StandardMacros.IsValid` OtherActor
    (:`Is Valid`
      (bind _asbp_player_character (cast `/Game/Blueprints/Player/BP_PlayerCharacter` OtherActor))
      (`/Game/Blueprints/Player/BP_PlayerCharacter.OverlappedInteractablesHandler` _asbp_player_character 1))))

(event `self.InformativeDetectableArea.OnComponentEndOverlap`
  (params (OverlappedComponent :type "PrimitiveComponent Object Reference") (OtherActor :type "Actor Object Reference") (OtherComp :type "PrimitiveComponent Object Reference") (OtherBodyIndex :type Integer))
  (`/Engine/EditorBlueprintResources/StandardMacros.IsValid` OtherActor
    (:`Is Valid`
      (bind _asbp_player_character (cast `/Game/Blueprints/Player/BP_PlayerCharacter` OtherActor))
      (`/Game/Blueprints/Player/BP_PlayerCharacter.OverlappedInteractablesHandler` _asbp_player_character -1))))

(fn `UserConstructionScript`
  (`parent.UserConstructionScript`))