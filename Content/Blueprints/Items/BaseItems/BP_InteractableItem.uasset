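; BP_InteractableItem is an item actor that players can detect as interactable when they come near it.
; On BeginPlay it passes itself to the WBP_InteractWidget in its InteractionWidget component as the item reference.
; Its InteractableDetectableArea reports overlaps to BP_PlayerCharacter's OverlappedInteractablesHandler, sending +1 on enter and -1 on exit.
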(event `self.ReceiveBeginPlay`
  (`parent.ReceiveBeginPlay`)
  (bind _aswbp_interact_widget (cast `/Game/Blueprints/HUDs/Gameplay/WBP_InteractWidget` (`WidgetComponent.GetUserWidgetObject` (`self.InteractionWidget`))))
  (set `/Game/Blueprints/HUDs/Gameplay/WBP_InteractWidget.ItemReference` self _aswbp_interact_widget))

(event `self.InteractableDetectableArea.OnComponentBeginOverlap`
  (params (OverlappedComponent :type "PrimitiveComponent Object Reference") (OtherActor :type "Actor Object Reference") (OtherComp :type "PrimitiveComponent Object Reference") (OtherBodyIndex :type Integer) (bFromSweep :type Boolean) (SweepResult :type "HitResult Structure (by ref)"))
  (`/Engine/EditorBlueprintResources/StandardMacros.IsValid` OtherActor
    (:`Is Valid`
      (bind _asbp_player_character (cast `/Game/Blueprints/Player/BP_PlayerCharacter` OtherActor))
      (`/Game/Blueprints/Player/BP_PlayerCharacter.OverlappedInteractablesHandler` _asbp_player_character 1))))

(event `self.InteractableDetectableArea.OnComponentEndOverlap`
  (params (OverlappedComponent :type "PrimitiveComponent Object Reference") (OtherActor :type "Actor Object Reference") (OtherComp :type "PrimitiveComponent Object Reference") (OtherBodyIndex :type Integer))
  (`/Engine/EditorBlueprintResources/StandardMacros.IsValid` OtherActor
    (:`Is Valid`
      (bind _asbp_player_character (cast `/Game/Blueprints/Player/BP_PlayerCharacter` OtherActor))
      (`/Game/Blueprints/Player/BP_PlayerCharacter.OverlappedInteractablesHandler` _asbp_player_character -1))))

(fn `UserConstructionScript`
  (`parent.UserConstructionScript`))