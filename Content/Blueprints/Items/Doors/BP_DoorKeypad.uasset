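; BP_DoorKeypad is a door keypad item that relays password entry to its on-screen keypad widget.
; KeyEntryHandler forwards keys to the WBP_KeypadEntry in its KeypadWidget component.
; PasswordCorrectHandler sets the PasswordCorrect flag and notifies the WBP_InteractWidget.
; When the player leaves the interactable detection area, it disables their password entry, clears their keypad reference and hides the keypad widget.
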(event `self.InteractableDetectableArea.OnComponentEndOverlap`
  (params (OverlappedComponent :type "PrimitiveComponent Object Reference") (OtherActor :type "Actor Object Reference") (OtherComp :type "PrimitiveComponent Object Reference") (OtherBodyIndex :type Integer))
  (bind _asbp_player_character (cast `/Game/Blueprints/Player/BP_PlayerCharacter` OtherActor))
  (set `/Game/Blueprints/Player/BP_PlayerCharacter.bCanEnterPassword` false _asbp_player_character)
  (set `/Game/Blueprints/Player/BP_PlayerCharacter.KeypadRef` null _asbp_player_character)
  (`SceneComponent.SetVisibility` (`self.KeypadWidget`) false false))

(fn `KeyEntryHandler`
  (params (Key :type Integer))
  (bind _aswbp_keypad_entry (cast `/Game/Blueprints/HUDs/WBP_KeypadEntry` (`WidgetComponent.GetUserWidgetObject` (`self.KeypadWidget`))))
  (`/Game/Blueprints/HUDs/WBP_KeypadEntry.KeyEntryHandler` _aswbp_keypad_entry Key))

(fn `PasswordCorrectHandler`
  (set `self.bPasswordCorrect` true)
  (bind _aswbp_interact_widget (cast `/Game/Blueprints/HUDs/WBP_InteractWidget` (`WidgetComponent.GetUserWidgetObject` (`self.InteractionWidget`))))
  (`/Game/Blueprints/HUDs/WBP_InteractWidget.Password Correct Handler` _aswbp_interact_widget))

(fn `UserConstructionScript`
  (`parent.UserConstructionScript`))