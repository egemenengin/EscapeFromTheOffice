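; BP_KeyDoor is a color-coded locked door that tells the player whether they carry the matching key.
; BeginPlay tints its sphere by KeyColor, and CheckKey searches the player's Keys for that color, latching HaveKey once found.
; While Locked, entering InteractableArea registers the door as the player's item target and shows a widget reflecting HaveKey.
; Leaving clears that registration and hides the widget; unlocking is not handled here.
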(event `self.ReceiveBeginPlay`
  (`parent.ReceiveBeginPlay`)
  (switch `/Game/Blueprints/EKeyColor` (`self.KeyColor`)
    (:`NewEnumerator0`
      (`PrimitiveComponent.SetMaterial` (`self.Sphere`) 0 "/Game/Materials/Key/M_Yellow.M_Yellow"))
    (:`NewEnumerator1`
      (`PrimitiveComponent.SetMaterial` (`self.Sphere`) 0 "/Game/Materials/Key/M_Blue.M_Blue"))
    (:`NewEnumerator2`
      (`PrimitiveComponent.SetMaterial` (`self.Sphere`) 0 "/Game/Materials/Key/M_Red.M_Red"))))

(event `self.InteractableArea.OnComponentBeginOverlap`
  (params (OverlappedComponent :type "PrimitiveComponent Object Reference") (OtherActor :type "Actor Object Reference") (OtherComp :type "PrimitiveComponent Object Reference") (OtherBodyIndex :type Integer) (bFromSweep :type Boolean) (SweepResult :type "HitResult Structure (by ref)"))
  ;[1 1 1] Comment
  (if (`self.bLocked`)
    (`/Engine/EditorBlueprintResources/StandardMacros.IsValid` OtherActor
      (:`Is Valid`
        (bind _asbp_player_character (cast `/Game/Blueprints/Player/BP_PlayerCharacter` OtherActor))
        (`self.CheckKey` _asbp_player_character)
        (set `/Game/Blueprints/Player/BP_PlayerCharacter.ItemRequiringDoor` self _asbp_player_character)
        (set `/Game/Blueprints/Player/BP_PlayerCharacter.bCanUseItem` true _asbp_player_character)
        (bind _aswbp_key_door_widget (cast `/Game/Blueprints/HUDs/WBP_KeyDoorWidget` (`WidgetComponent.GetUserWidgetObject` (`self.InteractWidget`))))
        (`/Game/Blueprints/HUDs/WBP_KeyDoorWidget.SetVisibilities` _aswbp_key_door_widget (`self.bHaveKey`))
        (`SceneComponent.SetVisibility` (`self.InteractWidget`) true false)))))

(event `self.InteractableArea.OnComponentEndOverlap`
  (params (OverlappedComponent :type "PrimitiveComponent Object Reference") (OtherActor :type "Actor Object Reference") (OtherComp :type "PrimitiveComponent Object Reference") (OtherBodyIndex :type Integer))
  ;[1 1 1] Comment
  (`/Engine/EditorBlueprintResources/StandardMacros.IsValid` OtherActor
    (:`Is Valid`
      (bind _asbp_player_character (cast `/Game/Blueprints/Player/BP_PlayerCharacter` OtherActor))
      (`self.CheckKey` _asbp_player_character)
      (set `/Game/Blueprints/Player/BP_PlayerCharacter.ItemRequiringDoor` null _asbp_player_character)
      (set `/Game/Blueprints/Player/BP_PlayerCharacter.bCanUseItem` false _asbp_player_character)
      (`SceneComponent.SetVisibility` (`self.InteractWidget`) false false))))

(fn `CheckKey`
  (params (Player :type "/Game/Blueprints/Player/BP_PlayerCharacter Object Reference"))
  (if (not (`self.bHaveKey`))
    (for _array_element (`/Game/Blueprints/Player/BP_PlayerCharacter.Keys` Player)
      (if (`|EnumEquality` (`/Game/Blueprints/Items/Doors/BP_Key.Color` _array_element) (`self.KeyColor`))
        (set `self.bHaveKey` true)
        (return)))))

(fn `UserConstructionScript`
  (`parent.UserConstructionScript`))