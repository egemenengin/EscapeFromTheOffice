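; BP_Door is a swinging door that opens itself while unlocked and closes when locked.
; Tick calls OpenDoor, which nudges the Door's world yaw each frame until its relative yaw reaches a threshold, then flips IsOpen.
; LeftHandle selects swing direction and limits.
; The step is delta time plus one, so speed depends on frame rate, and left-handed closing prints a debug string.
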(event `self.ReceiveTick`
  (params (DeltaSeconds :type "Float (single-precision)"))
  (`parent.ReceiveTick` DeltaSeconds)
  (`self.OpenDoor` DeltaSeconds))

(fn `OpenDoor`
  (params (DeltaSeconds :type "Float (double-precision)"))
  (bind _bisopen (`self.bIsOpen`))
  (bind _door (`self.Door`))
  (bind _door_2 (`self.Door`))
  (bind _door_3 (`self.Door`))
  (bind _door_4 (`self.Door`))
  (bind (_returnvalue_roll _returnvalue_pitch _returnvalue_yaw) (`KismetMathLibrary.BreakRotator` (`SceneComponent.K2_GetComponentRotation` _door_2)))
  (bind (_returnvalue_roll_2 _returnvalue_pitch_2 _returnvalue_yaw_2) (`KismetMathLibrary.BreakRotator` (`SceneComponent.K2_GetComponentRotation` _door_3)))
  (bind (_returnvalue_roll_3 _returnvalue_pitch_3 _returnvalue_yaw_3) (`KismetMathLibrary.BreakRotator` (`SceneComponent.K2_GetComponentRotation` _door_4)))
  (bind (_returnvalue_roll_4 _returnvalue_pitch_4 _returnvalue_yaw_4) (`KismetMathLibrary.BreakRotator` (`SceneComponent.K2_GetComponentRotation` _door)))
  (bind (_relativerotation_roll _relativerotation_pitch _relativerotation_yaw) (`KismetMathLibrary.BreakRotator` (`SceneComponent.RelativeRotation` (`self.Door`))))
  (set `self.DeltaSeconds` DeltaSeconds)
  (`/Engine/EditorBlueprintResources/StandardMacros.IncrementFloat` (`self.DeltaSeconds`)
    (:`  `
      (set `self.DoorYaw` _relativerotation_yaw)
      (if (not (`self.bLocked`))
        ;[1 1 1] Open Door
        (if _bisopen
          _
          (elif (`self.bLeftHandle`)
            ;;[1 1 1] If Left Handle
            (if (< (`self.DoorYaw`) -95.0)
              (`SceneComponent.K2_SetWorldRotation` _door_4 (`KismetMathLibrary.MakeRotator` _returnvalue_roll_3 _returnvalue_pitch_3 (+ _returnvalue_yaw_3 (`self.DeltaSeconds`))) false false)
              (else
                (set `self.bIsOpen` true)))
            (else
              ;;[1 1 1] If Right Handle
              (if (> (`self.DoorYaw`) -85.0)
                (`SceneComponent.K2_SetWorldRotation` _door_2 (`KismetMathLibrary.MakeRotator` _returnvalue_roll _returnvalue_pitch (- _returnvalue_yaw (`self.DeltaSeconds`))) false false)
                (else
                  (set `self.bIsOpen` true))))))
        (else
          ;[1 1 1] Close Door
          (if _bisopen
            (if (`self.bLeftHandle`)
              ;;[1 1 1] If Left Handle
              (if (> (`self.DoorYaw`) -175.0)
                (`SceneComponent.K2_SetWorldRotation` _door (`KismetMathLibrary.MakeRotator` _returnvalue_roll_4 _returnvalue_pitch_4 (- _returnvalue_yaw_4 (`self.DeltaSeconds`))) false false)
                (`KismetSystemLibrary.PrintString` "Hello")
                (else
                  (set `self.bIsOpen` false)))
              (else
                ;;[1 1 1] Right Handle
                (if (< (`self.DoorYaw`) 5.0)
                  (`SceneComponent.K2_SetWorldRotation` _door_3 (`KismetMathLibrary.MakeRotator` _returnvalue_roll_2 _returnvalue_pitch_2 (+ _returnvalue_yaw_2 (`self.DeltaSeconds`))) false false)
                  (else
                    (set `self.bIsOpen` false)))))))))))

(fn `UserConstructionScript`
  (`parent.UserConstructionScript`))