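; Door Blueprint that pairs with a child-actor keypad to use a password.
; On BeginPlay it casts the child BP_DoorKeypad and fetches the WBP_KeypadEntry from its widget component.
; It then hands that widget a reference to itself and its DoorPassword as the current password.
; Password checking and door opening are not handled in these graphs.
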(event `self.ReceiveBeginPlay`
  (`parent.ReceiveBeginPlay`)
  (bind _asbp_door_keypad (cast `/Game/Blueprints/Items/Doors/BP_DoorKeypad` (`ChildActorComponent.ChildActor` (`self.BP_DoorKeypad`))))
  (bind _aswbp_keypad_entry (cast `/Game/Blueprints/HUDs/WBP_KeypadEntry` (`WidgetComponent.GetUserWidgetObject` (`/Game/Blueprints/Items/Doors/BP_DoorKeypad.KeypadWidget` _asbp_door_keypad))))
  (set `/Game/Blueprints/HUDs/WBP_KeypadEntry.DoorRef` self _aswbp_keypad_entry)
  (set `/Game/Blueprints/HUDs/WBP_KeypadEntry.CurrentPassword` (`self.DoorPassword`) _aswbp_keypad_entry))

(fn `UserConstructionScript`
  (`parent.UserConstructionScript`))