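; BP_Key is a key item Blueprint, filed with the door items, that comes in yellow, blue or red.
; On BeginPlay it runs the parent logic, then switches on its Color value to apply the matching material to the StaticMesh.
; It adds no other behavior: the overlap and tick events are disabled and the construction script only calls its parent.
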(event `self.ReceiveBeginPlay`
  (`parent.ReceiveBeginPlay`)
  (switch `/Game/Blueprints/Enums/EKeyColor` (`self.Color`)
    (:`NewEnumerator0`
      (`PrimitiveComponent.SetMaterial` (`self.StaticMesh`) 0 "/Game/Materials/Key/M_Yellow.M_Yellow"))
    (:`NewEnumerator1`
      (`PrimitiveComponent.SetMaterial` (`self.StaticMesh`) 0 "/Game/Materials/Key/M_Blue.M_Blue"))
    (:`NewEnumerator2`
      (`PrimitiveComponent.SetMaterial` (`self.StaticMesh`) 0 "/Game/Materials/Key/M_Red.M_Red"))))

(fn `UserConstructionScript`
  (`parent.UserConstructionScript`))