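; BP_Lever is a lever actor that swings between an up and a down position.
; InteractLever only flips the IsUp flag, leaving the motion to RotateLever, which runs on BeginPlay and every Tick.
; RotateLever turns LeverCylinder in fixed one-degree local steps, tracking ChangedAmount to stop at either 45-degree limit.
; The step ignores DeltaSeconds, so swing speed depends on frame rate.
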(event `self.ReceiveBeginPlay`
  (`parent.ReceiveBeginPlay`)
  (`self.RotateLever`))

(event `self.ReceiveTick`
  (params (DeltaSeconds :type "Float (single-precision)"))
  (`parent.ReceiveTick` DeltaSeconds)
  (`self.RotateLever`))

(fn `InteractLever`
  (set `self.bIsUp` (not (`self.bIsUp`))))

(fn `RotateLever`
  (if (`self.bIsUp`)
    (if (> (`self.ChangedAmount`) -45)
      (`SceneComponent.K2_AddLocalRotation` (`self.LeverCylinder`) (struct :`Yaw` -1.0) false false)
      (`/Engine/EditorBlueprintResources/StandardMacros.DecrementInt` (`self.ChangedAmount`)))
    (elif (< (`self.ChangedAmount`) 45)
      (`SceneComponent.K2_AddLocalRotation` (`self.LeverCylinder`) (struct :`Yaw` 1.0) false false)
      (`/Engine/EditorBlueprintResources/StandardMacros.IncrementInt` (`self.ChangedAmount`)))))

(fn `UserConstructionScript`
  (`parent.UserConstructionScript`))