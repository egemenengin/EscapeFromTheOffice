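; Lever-puzzle door that unlocks when its eight levers match a set combination of up and down positions.
; BeginPlay casts eight child-actor levers to BP_Lever and stores them in an ordered array.
; While locked, Tick polls each lever's IsUp against RightAnswers, resetting the match count at the first mismatch and clearing Locked when the count reaches eight.
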(event `self.ReceiveBeginPlay`
  (`parent.ReceiveBeginPlay`)
  (`self.InitializeLeversArray`))

(event `self.ReceiveTick`
  (params (DeltaSeconds :type "Float (single-precision)"))
  (`parent.ReceiveTick` DeltaSeconds)
  (`self.CheckDoorIsOpen`))

(fn `CheckDoorIsOpen`
  (locals (NumCorrectAnswer :type Integer))
  (if (`self.bLocked`)
    (for (_array_element _array_index) (`self.RightAnswers`)
      (if (== _array_element (`/Game/Blueprints/Items/Doors/BP_Lever.bIsUp` (`|GetArrayItem` (`self.Levers`) _array_index)))
        (bind _result (`/Engine/EditorBlueprintResources/StandardMacros.IncrementInt` (`local.NumCorrectAnswer`))
          (:`  `
            (if (== _result 8)
              (set `self.bLocked` false)
              (else
                (set `self.bLocked` true)))))
        (else
          (set `local.NumCorrectAnswer` 0)
          (break))))))

(fn `InitializeLeversArray`
  (bind _asbp_lever (cast `/Game/Blueprints/Items/Doors/BP_Lever` (`ChildActorComponent.ChildActor` (`self.Lever1`))))
  (`KismetArrayLibrary.Array_Add` (`self.Levers`) _asbp_lever)
  (bind _asbp_lever_2 (cast `/Game/Blueprints/Items/Doors/BP_Lever` (`ChildActorComponent.ChildActor` (`self.Lever2`))))
  (`KismetArrayLibrary.Array_Add` (`self.Levers`) _asbp_lever_2)
  (bind _asbp_lever_3 (cast `/Game/Blueprints/Items/Doors/BP_Lever` (`ChildActorComponent.ChildActor` (`self.Lever3`))))
  (`KismetArrayLibrary.Array_Add` (`self.Levers`) _asbp_lever_3)
  (bind _asbp_lever_4 (cast `/Game/Blueprints/Items/Doors/BP_Lever` (`ChildActorComponent.ChildActor` (`self.Lever4`))))
  (`KismetArrayLibrary.Array_Add` (`self.Levers`) _asbp_lever_4)
  (bind _asbp_lever_5 (cast `/Game/Blueprints/Items/Doors/BP_Lever` (`ChildActorComponent.ChildActor` (`self.Lever5`))))
  (`KismetArrayLibrary.Array_Add` (`self.Levers`) _asbp_lever_5)
  (bind _asbp_lever_6 (cast `/Game/Blueprints/Items/Doors/BP_Lever` (`ChildActorComponent.ChildActor` (`self.Lever6`))))
  (`KismetArrayLibrary.Array_Add` (`self.Levers`) _asbp_lever_6)
  (bind _asbp_lever_7 (cast `/Game/Blueprints/Items/Doors/BP_Lever` (`ChildActorComponent.ChildActor` (`self.Lever7`))))
  (`KismetArrayLibrary.Array_Add` (`self.Levers`) _asbp_lever_7)
  (bind _asbp_lever_8 (cast `/Game/Blueprints/Items/Doors/BP_Lever` (`ChildActorComponent.ChildActor` (`self.Lever8`))))
  (`KismetArrayLibrary.Array_Add` (`self.Levers`) _asbp_lever_8))

(fn `UserConstructionScript`
  (`parent.UserConstructionScript`))