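; Pressure plate door that a player character unlocks by stepping on the plate.
; Overlapping the plate's collision clears Locked, lowers the plate mesh slightly and switches it to the enabled material.
; Leaving starts a fixed delay, then relocks, raises the plate and restores the disabled material, without rechecking whether the player has returned.
; Door movement is not handled in this graph, which only toggles Locked and calls parent BeginPlay and construction logic.
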(event `self.ReceiveBeginPlay`
  (`parent.ReceiveBeginPlay`))

(event `self.PressurePlateCollision.OnComponentBeginOverlap`
  (params (OverlappedComponent :type "PrimitiveComponent Object Reference") (OtherActor :type "Actor Object Reference") (OtherComp :type "PrimitiveComponent Object Reference") (OtherBodyIndex :type Integer) (bFromSweep :type Boolean) (SweepResult :type "HitResult Structure (by ref)"))
  (bind (_returnvalue_x _returnvalue_y _returnvalue_z) (`KismetMathLibrary.BreakVector` (`SceneComponent.K2_GetComponentLocation` (`self.PressurePlate`))))
  (`/Engine/EditorBlueprintResources/StandardMacros.IsValid` OtherActor
    (:`Is Valid`
      (cast `/Game/Blueprints/Player/BP_PlayerCharacter` OtherActor)
      (if (`self.bLocked`)
        (set `self.bLocked` false)
        (`SceneComponent.K2_SetWorldLocation` (`self.PressurePlate`) (`KismetMathLibrary.MakeVector` _returnvalue_x _returnvalue_y (- _returnvalue_z 3.0)) false false)
        (`PrimitiveComponent.SetMaterial` (`self.PressurePlate`) 0 "/Game/Materials/Door/M_PressurePlateEnabled.M_PressurePlateEnabled")))))

(event `self.PressurePlateCollision.OnComponentEndOverlap`
  (params (OverlappedComponent :type "PrimitiveComponent Object Reference") (OtherActor :type "Actor Object Reference") (OtherComp :type "PrimitiveComponent Object Reference") (OtherBodyIndex :type Integer))
  (bind (_returnvalue_x _returnvalue_y _returnvalue_z) (`KismetMathLibrary.BreakVector` (`SceneComponent.K2_GetComponentLocation` (`self.PressurePlate`))))
  (`/Engine/EditorBlueprintResources/StandardMacros.IsValid` OtherActor
    (:`Is Valid`
      (cast `/Game/Blueprints/Player/BP_PlayerCharacter` OtherActor)
      (`KismetSystemLibrary.Delay` 5.0)
      (if (not (`self.bLocked`))
        (set `self.bLocked` true)
        (`SceneComponent.K2_SetWorldLocation` (`self.PressurePlate`) (`KismetMathLibrary.MakeVector` _returnvalue_x _returnvalue_y (+ _returnvalue_z 3.0)) false false)
        (`PrimitiveComponent.SetMaterial` (`self.PressurePlate`) 0 "/Game/Materials/Door/M_PressurePlateDisabled.M_PressurePlateDisabled")))))

(fn `UserConstructionScript`
  (`parent.UserConstructionScript`))