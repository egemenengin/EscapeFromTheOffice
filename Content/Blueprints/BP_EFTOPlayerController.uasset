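; Player controller for EFTO that runs each floor's countdown and drives the game status: alive, paused, caught, time up or finished.
; BeginPlay loads save data from the game instance, sets the time by map name, creates the HUD and starts a one-second timer that ends the run at zero.
; SetGameStatus switches panels, input mode and cursor, disabling the character on end states.
; Finishing a floor saves unlock progress and shows the level-finished or game-end widget.
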(event `self.ReceiveBeginPlay`
  (bind _asbp_efto_game_instance (cast `/Game/Blueprints/BP_EFTO_GameInstance` (`GameplayStatics.GetGameInstance`)))
  (set `self.PlayerPreferences` (`/Game/Blueprints/BP_EFTO_GameInstance.SaveGameData` _asbp_efto_game_instance))
  (set `self.SaveSlotName` (`/Game/Blueprints/BP_EFTO_GameInstance.SaveSlotName` _asbp_efto_game_instance))
  (`self.SetCurrentLevelTime`)
  (bind _returnvalue (`|CreateWidget` "/Game/Blueprints/HUDs/Gameplay/WBP_PlayerHUD.WBP_PlayerHUD_C"))
  (bind _aswbp_player_hud (cast `/Game/Blueprints/HUDs/Gameplay/WBP_PlayerHUD` _returnvalue))
  (bind _output_get (set `self.PlayerHUD` _aswbp_player_hud))
  (`UserWidget.AddToViewport` _output_get 0)
  (`/Game/Blueprints/HUDs/Gameplay/WBP_RemainingTime.TimeHandler` (`/Game/Blueprints/HUDs/Gameplay/WBP_PlayerHUD.WBP_RemainingTime` _output_get) (`self.CurrentLevelTime`))
  (`KismetSystemLibrary.K2_SetTimer` null "TimeHandler" 1.0 true))

(event `EnhancedInput|/Game/Blueprints/Player/Input/InputActions/IA_PauseGame`
  (params (ActionValue :type Boolean) (ElapsedSeconds :type "Float (double-precision)") (TriggeredSeconds :type "Float (double-precision)") (InputAction :type "InputAction Object Reference" :default "/Game/Blueprints/Player/Input/InputActions/IA_PauseGame.IA_PauseGame"))
  (:`Triggered`
    (`self.SetGameStatus` "NewEnumerator1")))

(fn `HandlePlayerLastUnlockedLevel`
  (params (FinishedFloor :type Integer))
  (bind _playerpreferences (`self.PlayerPreferences`))
  (if (> FinishedFloor (`/Game/Blueprints/BP_PlayerPreferences.LastUnlockedLevel` (`self.PlayerPreferences`)))
    (set `/Game/Blueprints/BP_PlayerPreferences.LastUnlockedLevel` FinishedFloor _playerpreferences)
    (`GameplayStatics.SaveGameToSlot` _playerpreferences (`self.SaveSlotName`))))

(fn `HandleWinWidget`
  (params (FinishedLevel :type Integer))
  (locals (FinishedFloor :type Integer))
  (set `local.FinishedFloor` FinishedLevel)
  (if (< FinishedLevel 2)
    (bind _returnvalue (`|CreateWidget` "/Game/Blueprints/HUDs/Menu/LevelEndPanels/WBP_LevelFinished.WBP_LevelFinished_C"))
    (set `/Game/Blueprints/HUDs/Menu/LevelEndPanels/WBP_LevelFinished.FinishedFloor` (`local.FinishedFloor`) _returnvalue)
    (`UserWidget.AddToViewport` _returnvalue 0)
    (else
      (bind _returnvalue_2 (`|CreateWidget` "/Game/Blueprints/HUDs/Menu/LevelEndPanels/WBP_GameEndPanel.WBP_GameEndPanel_C"))
      (`UserWidget.AddToViewport` _returnvalue_2 0))))

(fn `SetCurrentLevelTime`
  (bind _returnvalue (`GameplayStatics.GetCurrentLevelName` true))
  (switch `string` _returnvalue
    (:`ThirdFloorMap`
      (set `self.CurrentLevelTime` 120))
    (:`SecondFloorMap`
      (set `self.CurrentLevelTime` 120))
    (:`FirstFloorMap`
      (set `self.CurrentLevelTime` 120))))

(fn `SetGameStatus`
  (params (NewGameStatus :type "/Game/Blueprints/Enums/EGameStatus Enum" :default "NewEnumerator0") (FinishedFloor :type Integer))
  (bind _returnvalue (`GameplayStatics.GetPlayerCharacter` 0))
  (bind _output_get (set `self.GameStatus` NewGameStatus))
  (switch `/Game/Blueprints/Enums/EGameStatus` _output_get
    (:`NewEnumerator0`
      (`/Engine/EditorBlueprintResources/StandardMacros.IsValid` (`self.PausePanel`)
        (:`Is Valid`
          (`Widget.SetVisibility` (`self.PausePanel`) "Hidden"))
        (:`Is Not Valid`
          _))
      (`WidgetBlueprintLibrary.SetInputMode_GameOnly` self)
      (set `self.bShowMouseCursor` false))
    (:`NewEnumerator1`
      (`/Engine/EditorBlueprintResources/StandardMacros.IsValid` (`self.PausePanel`)
        (:`Is Valid`
          (`Widget.SetVisibility` (`self.PausePanel`) "Visible"))
        (:`Is Not Valid`
          (bind _returnvalue_2 (`|CreateWidget` "/Game/Blueprints/HUDs/Menu/WBP_PausePanel.WBP_PausePanel_C"))
          (`UserWidget.AddToViewport` _returnvalue_2 0)
          (set `self.PausePanel` _returnvalue_2)))
      (`WidgetBlueprintLibrary.SetInputMode_UIOnlyEx` self _returnvalue_2)
      (set `self.bShowMouseCursor` true))
    (:`NewEnumerator3`
      (bind _returnvalue_3 (`|CreateWidget` "/Game/Blueprints/HUDs/Menu/LevelEndPanels/WBP_CaughtPanel.WBP_CaughtPanel_C"))
      (`UserWidget.AddToViewport` _returnvalue_3 0)
      (`WidgetBlueprintLibrary.SetInputMode_UIOnlyEx` self null :!label _label)
      (set `self.bShowMouseCursor` true)
      (`Widget.RemoveFromParent` (`self.PlayerHUD`))
      (`CharacterMovementComponent.DisableMovement` (`Character.CharacterMovement` _returnvalue))
      (`PrimitiveComponent.SetCollisionEnabled` (`Character.CapsuleComponent` _returnvalue) "NoCollision"))
    (:`NewEnumerator4`
      (bind _returnvalue_4 (`|CreateWidget` "/Game/Blueprints/HUDs/Menu/LevelEndPanels/WBP_TimesUp.WBP_TimesUp_C"))
      (`UserWidget.AddToViewport` _returnvalue_4 0)
      (goto _label))
    (:`NewEnumerator2`
      (`self.HandlePlayerLastUnlockedLevel` FinishedFloor)
      (`self.HandleWinWidget` FinishedFloor)
      (goto _label))))

(fn `TimeHandler`
  (if (`|EnumEquality` (`self.GameStatus`) "NewEnumerator0")
    (`/Engine/EditorBlueprintResources/StandardMacros.DecrementInt` (`self.CurrentLevelTime`)
      (:`  `
        (`/Game/Blueprints/HUDs/Gameplay/WBP_RemainingTime.TimeHandler` (`/Game/Blueprints/HUDs/Gameplay/WBP_PlayerHUD.WBP_RemainingTime` (`self.PlayerHUD`)) (`self.CurrentLevelTime`))
        (if (<= (`self.CurrentLevelTime`) 0)
          (`self.SetGameStatus` "NewEnumerator4"))))))

(fn `UserConstructionScript`)